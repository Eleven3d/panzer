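; Weapon scene component that fires a bullet actor from its own world location and rotation, owned by the component's owner.
; Shoot casts the spawn to BP_Bullet, sets its velocity along the component's forward vector and broadcasts OnBulletSpawned.
; The velocity magnitude sums squared BulletVelocity and the squared speed of the owner's BAC_SplineTracer, if present, with no square root taken.
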(fn Shoot
  (bind _returnvalue (Transformation|GetWorldTransform))
  (bind _returnvalue_2 (Game|SpawnActorfromClass (Variables|Default|GetBullet) (Math|Transform|MakeTransform (.location _returnvalue) (.rotation _returnvalue)) "AdjustIfPossibleButAlwaysSpawn" (Components|GetOwner) 0))
  (bind _asbp_bullet (Utilities|Casting|CastToBP_Bullet _returnvalue_2))
  (Default|SetVelocity _asbp_bullet (* (Math|Vector|GetForwardVector (Transformation|GetWorldRotation)) (+ (Math|Float|Square (Variables|Default|GetBulletVelocity)) (CallFunction|GetInheritedVelocity))))
  (Default|CallOnBulletSpawned _asbp_bullet))

(fn GetInheritedVelocity
  (bind _returnvalue (Components|GetOwner))
  (bind _returnvalue_2 (Actor|GetComponentbyClass _returnvalue "/Game/Blueprints/Spline/BAC_SplineTracer.BAC_SplineTracer_C"))
  (Utilities|IsValid _returnvalue_2
    (:Is%20Valid
      (return (Math|Vector|VectorLengthSquared (Default|GetVelocity _returnvalue_2))))
    (:Is%20Not%20Valid
      (return 0.0))))