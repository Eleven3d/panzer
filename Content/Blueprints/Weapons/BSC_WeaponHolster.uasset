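; Weapon holster scene component that spawns a weapon at its transform on BeginPlay, attached to the holster's parent with physics off.
; Spawning also sets up grip-release bindings on the weapon's BAC_Grabbable component.
; The release handler destroys the weapon and starts a one-shot timeout timer, which the grab handler clears.
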(event Custom|OnWeaponReleased
  (params (BSCMotionController :type BSC%20Motion%20Controller%20Object%20Reference))
  (Actor|DestroyActor (Variables|Default|GetSpawnedWeapon))
  (bind _returnvalue (Utilities|Time|SetTimerbyEvent (EventDispatchers|CreateEvent :!event SpawnWeapon) (Variables|Default|GetTimeoutDelay)))
  (Variables|Default|SetWeaponTimeoutHandle _returnvalue))

(event Custom|OnWeaponGrabbed
  (params (BSCMotionController :type BSC%20Motion%20Controller%20Object%20Reference))
  (Utilities|Time|ClearandInvalidateTimerbyHandle (Variables|Default|GetWeaponTimeoutHandle)))

(event EventBeginPlay
  (CallFunction|SpawnWeapon))

(fn SpawnWeapon
  (bind _returnvalue (Game|SpawnActorfromClass (Variables|Default|GetWeapon) (Transformation|GetWorldTransform) "AlwaysSpawn" (Components|GetOwner) 0))
  (bind _output_get (Variables|Default|SetSpawnedWeapon _returnvalue))
  (Transformation|AttachComponentToComponent _output_get (Transformation|GetAttachParent) "None" "KeepWorld" "KeepWorld" "KeepWorld" true)
  (EventDispatchers|BindEventtoOnGripReleasedEvent (Actor|GetComponentbyClass (Variables|Default|GetSpawnedWeapon) "/Game/Blueprints/Player/BAC_Grabbable.BAC_Grabbable_C") (EventDispatchers|CreateEvent :!event Custom|OnWeaponReleased))
  (EventDispatchers|UnbindEventfromOnGripReleasedEvent (Actor|GetComponentbyClass (Variables|Default|GetSpawnedWeapon) "/Game/Blueprints/Player/BAC_Grabbable.BAC_Grabbable_C") (EventDispatchers|CreateEvent :!event Custom|OnWeaponGrabbed))
  (bind _asprimitive_component (Utilities|Casting|CastToPrimitiveComponent (Variables|/Script/Engine.Actor|GetRootComponent (Variables|Default|GetSpawnedWeapon))))
  (Physics|SetSimulatePhysics _asprimitive_component false))