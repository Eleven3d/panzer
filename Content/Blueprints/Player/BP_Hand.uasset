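; BP_Hand is a motion-controlled player hand with an animated mesh and a grab volume.
; Construction registers the hand mesh and overlap volume with the BSC motion controller component as its hand and grab primitives.
; A single mesh serves both hands, with the left motion source inverting its Y scale to mirror it.
; The controller's hand state updates are forwarded to ABP_Hand to drive animation.
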(event OnHandStateUpdated(BSC_MotionController)
  (params (NewHandState :type E_HandState%20Enum :default "NewEnumerator0"))
  (bind _asabp_hand (Utilities|Casting|CastToABP_Hand (Components|SkeletalMesh|GetAnimInstance (Variables|Default|GetHandMesh))))
  (Default|UpdateHandState _asabp_hand NewHandState))

(fn ConstructionScript
  (CallFunction|SetMotionSourceVisual)
  (Default|SetHandPrimitive (Variables|Default|GetBSC_MotionController) (Variables|Default|GetHandMesh))
  (Default|SetGrabPrimitive (Variables|Default|GetBSC_MotionController) (Variables|Default|GetHandOverlapVolume)))

(fn SetMotionSourceVisual
  (bind _handmesh (Variables|Default|GetHandMesh))
  (bind _returnvalue (Transformation|GetWorldScale _handmesh))
  (switch Utilities|FlowControl|Switch|SwitchonE_MotionSource (Variables|Default|GetMotionSource)
    (:NewEnumerator0
      (Transformation|SetWorldScale3D (Variables|Default|GetHandMesh) (Math|Vector|MakeVector (.x _returnvalue) (CallFunction|InvertFloat (.y _returnvalue)) (.z _returnvalue))))))