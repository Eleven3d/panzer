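; BAC_Interactable is a component that tracks which motion controller currently owns an interaction with it.
; On receiving an interaction it notifies any existing owner that it was overwritten, stores the new controller and calls OnInteractionReceived.
; On release it clears the owner unconditionally and calls OnInteractionReleased with the releasing controller.
; It also exposes a setter and getter for its interaction primitives.
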(event Custom|InteractionReceived
  (params (BSCMotionController :type BSC%20Motion%20Controller%20Object%20Reference))
  (Utilities|IsValid (Variables|Interaction|GetCurrentOwner)
    (:Is%20Valid
      (Default|OnInteractableOverwritten (Variables|Interaction|GetCurrentOwner)))
    (:Is%20Not%20Valid
      _))
  (bind _output_get (Variables|Interaction|SetCurrentOwner BSCMotionController))
  (Default|CallOnInteractionReceived _output_get))

(event Custom|InteractionReleased
  (params (BSCMotionController :type BSC%20Motion%20Controller%20Object%20Reference))
  (Variables|Interaction|SetCurrentOwner 0)
  (Default|CallOnInteractionReleased BSCMotionController))

(fn SetInteractionPrimitives
  (params (InteractionPrimitive :type Array%20of%20Primitive%20Component%20Object%20References))
  (Variables|Interaction|SetInteractionPrimitive InteractionPrimitive))

(fn GetInteractionPrimitives
  (return (Variables|Interaction|GetInteractionPrimitive)))