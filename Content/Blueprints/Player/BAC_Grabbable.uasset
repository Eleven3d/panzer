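; BAC_Grabbable is a grip-handling component that lets a motion controller grab and carry the actor that owns it.
; On grip, it runs the parent handler, stores the controller and attaches the owner to it, keeping world transforms.
; On release, it clears that reference and detaches the owner in place.
; Two getters expose whether it is held and by which controller.
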(event EventGripReleased
  (params (BSCMotionController :type BSC%20Motion%20Controller%20Object%20Reference))
  (|CallParentFunction BSCMotionController)
  (Variables|Default|SetOwningMotionController 0)
  (Transformation|DetachFromActor (Components|GetOwner) "KeepWorld" "KeepWorld" "KeepWorld"))

(event EventGripReceived
  (params (BSCMotionController :type BSC%20Motion%20Controller%20Object%20Reference))
  (|CallParentFunction BSCMotionController)
  (Variables|Default|SetOwningMotionController BSCMotionController)
  (Transformation|AttachComponentToComponent (Components|GetOwner) BSCMotionController "None" "KeepWorld" "KeepWorld" "KeepWorld" true))

(fn IsGrabbed
  (return (Utilities|IsValid (Variables|Default|GetOwningMotionController))))

(fn GetGrabbingMotionController
  (return (Variables|Default|GetOwningMotionController)))