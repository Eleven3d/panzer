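; BP_Reigns is a grippable reins actor that turns motion controller pulls into a direction vector.
; Grip and release events track the interacting controllers and enable Tick only while any hold on.
; Tick sets the Reigns component's relative location from actor location minus the average controller location, through a clamp.
; GetReignsDirection uses a per-axis deadzone macro, signing each step by DeadzoneRadius rather than pull direction.
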(event OnGripEvent(BAC_Interactable)
  (params (BSCMotionController :type BSC%20Motion%20Controller%20Object%20Reference))
  (Utilities|Array|AddUnique (Variables|Default|GetInteractingMotioncontrollers) BSCMotionController)
  (CallFunction|UpdateTickEnabled))

(event OnGripReleasedEvent(BAC_Interactable)
  (params (BSCMotionController :type BSC%20Motion%20Controller%20Object%20Reference))
  (Utilities|Array|RemoveItem (Variables|Default|GetInteractingMotioncontrollers) BSCMotionController)
  (CallFunction|UpdateTickEnabled))

(event EventTick
  (params (DeltaSeconds :type Float%20%28single-precision%29))
  (Transformation|SetRelativeLocation (Variables|Default|GetReigns) (Class|BDUtilityLibrary|ClampVector (- (Transformation|GetActorLocation) (Class|BDUtilityLibrary|GetAverageWorldLocation (Variables|Default|GetInteractingMotioncontrollers))) "25.000000,25.000000,25.000000" "-25.000000,-25.000000,-5.000000") false false))

(fn ConstructionScript
  (Default|SetInteractionPrimitives (Variables|Default|GetBAC_Interactable) (Utilities|Array|MakeArray (Variables|Default|GetReigns))))

(fn GetReignsDirection
  (Utilities|HandleReignDirection (Variables|/Script/Engine.SceneComponent|GetRelativeLocation (Variables|Default|GetReigns))
    (:UpdateX
      (CallFunction|AddVector (LocalVariables|GetLocalReignDirection) (Math|Vector|MakeVector (CallFunction|GetAddedValue) 0.0 0.0)))
    (:UpdateY
      (CallFunction|AddVector (LocalVariables|GetLocalReignDirection) (Math|Vector|MakeVector 0.0 (CallFunction|GetAddedValue) 0.0)))
    (:UpdateZ
      (CallFunction|AddVector (LocalVariables|GetLocalReignDirection) (Math|Vector|MakeVector 0.0 0.0 (CallFunction|GetAddedValue))))
    (:Completed
      (return (LocalVariables|GetLocalReignDirection)))))

(fn GetAddedValue
  (return (select (>= (Variables|Default|GetDeadzoneRadius) 0.0) 1.0 -1.0)))

(fn UpdateTickEnabled
  (Actor|Tick|SetActorTickEnabled (> (Utilities|Array|Length (Variables|Default|GetInteractingMotioncontrollers)) 0)))