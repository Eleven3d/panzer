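; Motion controller component for the player's hand that drives a lagging hand visual and handles trigger-based interaction.
; Each tick interpolates the assigned hand primitive toward the controller's transform.
; Trigger press notifies the BAC_Interactable nearest the hand among grab-primitive overlaps; release or overwrite clears it.
; These events update and broadcast the hand state, while grip, face and home button handlers are empty.
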(event Custom|OnHomeButtonPressed)

(event Custom|OnFaceButton1Released)

(event Custom|OnFaceButton1Pressed)

(event Custom|OnTriggerReleased
  (Interaction|Release)
  (CallFunction|UpdateHandState "NewEnumerator0"))

(event Custom|OnFaceButton2Pressed)

(event Custom|OnTriggerPressed
  (bind _succesful (Interaction|Interact))
  (if _succesful
    (CallFunction|UpdateHandState "NewEnumerator2")
    (else
      (CallFunction|UpdateHandState "NewEnumerator1"))))

(event Custom|OnInteractableOverwritten
  (CallFunction|UpdateHandState (Utilities|Select :Index (Variables|Default|GetHandState) :NewEnumerator0 "NewEnumerator0" :NewEnumerator1 "NewEnumerator0" :NewEnumerator2 "NewEnumerator1" :NewEnumerator3 "NewEnumerator3" :NewEnumerator4 "NewEnumerator4"))
  (Variables|Default|SetCurrentInteractable 0))

(event Custom|OnGripPressed)

(event Custom|OnGripReleased)

(event Custom|OnFaceButton2Released)

(event EventTick
  (params (DeltaSeconds :type Float%20%28single-precision%29))
  (HandVisual|LerpHandTransform))

(event EventBeginPlay
  (Default|CallOnHandStateUpdated (Variables|Default|GetHandState)))

(fn SetHandPrimitive
  (params (Primitive :type Primitive%20Component%20Object%20Reference))
  (Variables|Default|SetHandVisual Primitive))

(fn SetGrabPrimitive
  (params (Primitives :type Primitive%20Component%20Object%20Reference))
  (Variables|Default|SetGrabPrimitive Primitives))

(fn GetHandTransform
  (return (Class|KismetMathLibrary|TInterpto (Transformation|GetWorldTransform (Variables|Default|GetHandVisual)) (Transformation|GetWorldTransform) (Utilities|Time|GetWorldDeltaSeconds) (Variables|Default|GetHandLerpSpeed))))

(fn LerpHandTransform
  (Utilities|IsValid (Variables|Default|GetHandVisual)
    (:Is%20Valid
      (Transformation|SetWorldTransform (Variables|Default|GetHandVisual) (HandVisual|GetHandTransform) false false))))

(fn Interact
  (for _array_element (Collision|GetOverlappingActors (Variables|Default|GetGrabPrimitive) "/Script/Engine.Actor" :!class /Script/Engine.PrimitiveComponent)
    (Utilities|IsValid (Actor|GetComponentbyClass _array_element "/Game/Blueprints/Player/BAC_Interactable.BAC_Interactable_C")
      (:Is%20Valid
        (Utilities|Array|Add (LocalVariables|GetInteractPrimitives) (Variables|/Game/Blueprints/Player/BAC_Interactable.BAC_Interactable_C|GetInteractionPrimitive (Actor|GetComponentbyClass _array_element "/Game/Blueprints/Player/BAC_Interactable.BAC_Interactable_C"))))))
  (if (> (Utilities|Array|Length (LocalVariables|GetInteractPrimitives)) 0)
    (bind _output_get (Variables|Default|SetCurrentInteractable (Actor|GetComponentbyClass (Components|GetOwner (Class|BDUtilityLibrary|GetNearestPrimitive (LocalVariables|GetInteractPrimitives) (Variables|Default|GetHandVisual))) "/Game/Blueprints/Player/BAC_Interactable.BAC_Interactable_C")))
    (Default|OnInteractionReceived _output_get self)
    (return true)
    (else
      (return false))))

(fn UpdateHandState
  (params (HandState :type E_HandState%20Enum :default "NewEnumerator0"))
  (bind _output_get (Variables|Default|SetHandState HandState))
  (Default|CallOnHandStateUpdated _output_get))

(fn Release
  (Utilities|IsValid (Variables|Default|GetCurrentInteractable)
    (:Is%20Valid
      (Default|OnInteractionReleased (Variables|Default|GetCurrentInteractable) self)
      (Variables|Default|SetCurrentInteractable 0))))