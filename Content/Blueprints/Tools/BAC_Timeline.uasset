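; Actor component that works as a reusable timeline, with play, reverse, stop and set-time controls.
; Tick advances a normalized time by delta over Duration in the current direction and broadcasts updates with time in seconds, an optional float curve's value and direction.
; When time leaves the 0–1 range, it restarts in the same direction if looping, otherwise disables its tick and broadcasts completion.
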(event EventTick
  (params (DeltaSeconds :type Float%20%28single-precision%29))
  (CallFunction|AddFloat (Variables|Parameters|GetInTime) (Lerp|GetNewTime))
  (if (Lerp|IsCompleted)
    (if (Variables|Parameters|GetLooping)
      (switch Utilities|FlowControl|Switch|SwitchonETimelineDirection (Variables|Timeline|GetDirection)
        (:Forward
          (Timeline|PlayfromStart))
        (:Backward
          (Timeline|ReversefromEnd)))
      (else
        (Dispatchers|CompleteTimeline)))
    (else
      (Dispatchers|UpdateTimeline))))

(fn PlayfromStart
  (Variables|Parameters|SetInTime 0.0)
  (Components|Tick|SetComponentTickEnabled true)
  (Variables|Timeline|SetDirection "Forward"))

(fn Play
  (Components|Tick|SetComponentTickEnabled true)
  (Variables|Timeline|SetDirection "Forward"))

(fn Stop
  (Components|Tick|SetComponentTickEnabled false))

(fn Reverse
  (Components|Tick|SetComponentTickEnabled true)
  (Variables|Timeline|SetDirection "Backward"))

(fn ReversefromEnd
  (Variables|Parameters|SetInTime 1.0)
  (Components|Tick|SetComponentTickEnabled true)
  (Variables|Timeline|SetDirection "Backward"))

(fn GetNewTime
  (return (/ (* (Utilities|Time|GetWorldDeltaSeconds) (Utilities|Select :Index (Variables|Timeline|GetDirection) :Forward 1.0 :Backward -1.0)) (Variables|Parameters|GetDuration))))

(fn IsCompleted
  (return (.WasClamped (CallFunction|ClampFloatChecked (Variables|Parameters|GetInTime) 0.0 1.0))))

(fn UpdateTimeline
  (Default|CallOnTimelineUpdated (ReturnValues|GetCurrentTime) (ReturnValues|GetCurveValue) (Variables|Timeline|GetDirection)))

(fn CompleteTimeline
  (Components|Tick|SetComponentTickEnabled false)
  (Default|CallOnTimelineCompleted (ReturnValues|GetCurrentTime) (ReturnValues|GetCurveValue) (Variables|Timeline|GetDirection)))

(fn SetNewTime
  (params (InTime :type Float%20%28single-precision%29))
  (Variables|Parameters|SetInTime (Math|Float|Clamp(Float) InTime)))

(fn GetCurveValue
  (bind _floatcurve (Variables|Parameters|GetFloatCurve))
  (Utilities|IsValid _floatcurve
    (:Is%20Valid
      (return (Math|Curves|GetFloatValue _floatcurve (Variables|Parameters|GetInTime))))
    (:Is%20Not%20Valid
      (return 0.0))))

(fn GetCurrentTime
  (return (Math|Float|Clamp(Float) (* (Variables|Parameters|GetInTime) (Variables|Parameters|GetDuration)) 0.0 (Variables|Parameters|GetDuration))))