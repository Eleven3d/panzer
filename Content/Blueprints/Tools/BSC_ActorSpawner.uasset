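; BSC_ActorSpawner is a scene component that spawns an actor of a configurable class at its own world transform.
; Spawning runs on BeginPlay when SpawnOnBeginPlay is set, or through SpawnActor, and always spawns, adjusting for collisions if possible.
; The new actor is stored, snapped and attached to the component, then broadcast through the OnActorSpawned dispatcher.
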(event EventBeginPlay
  (if (Variables|Default|GetSpawnOnBeginPlay)
    (CallFunction|SpawnActor)))

(fn SpawnActor
  (bind _returnvalue (Game|SpawnActorfromClass (Variables|Default|GetActorToSpawn) (Transformation|GetWorldTransform) "AdjustIfPossibleButAlwaysSpawn" 0 0))
  (bind _output_get (Variables|Default|SetSpawnedActor _returnvalue))
  (Transformation|AttachComponentToComponent _output_get self "None" "SnapToTarget" "SnapToTarget" "SnapToTarget" true)
  (Default|CallOnActorSpawned (Variables|Default|GetSpawnedActor)))