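; Game mode Blueprint that starts gameplay and advances game stages based on the Dragoon's movement along a spline.
; On BeginPlay it binds to the destination-reached event of the Dragoon's spline tracer component, then starts gameplay after a short delay.
; Starting gameplay updates the game state and sends the Dragoon along its target spline.
; The destination-reached handler tells the game state to move to the next stage.
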(event Custom|StartGameplay
  (bind _dragoon (CallFunction|GetDragoon))
  (Default|UpdateGameState (CallFunction|GetBPGameState) "NewEnumerator0")
  (Default|TraceSpline (Variables|/Game/Blueprints/Player/BP_Dragoon.BP_Dragoon_C|GetBAC_DragonSplineTracer _dragoon) (Default|GetTargetSpline _dragoon)))

(event Custom|OnDragoonSplineDestinationReached
  (Default|NextStage (CallFunction|GetBPGameState)))

(event EventBeginPlay
  (EventDispatchers|BindEventtoOnSplineDestinationReached (Variables|/Game/Blueprints/Player/BP_Dragoon.BP_Dragoon_C|GetBAC_DragonSplineTracer (CallFunction|GetDragoon)) (EventDispatchers|CreateEvent :!event Custom|OnDragoonSplineDestinationReached))
  (Utilities|FlowControl|Delay 2.0)
  (CallFunction|StartGameplay))

(fn ConstructionScript)