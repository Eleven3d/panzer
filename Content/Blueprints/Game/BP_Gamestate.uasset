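; BP_Gamestate tracks the current game state enum and stage index for the game.
; BeginPlay sets the initial state through UpdateGameState and resets the stage index to zero.
; UpdateGameState broadcasts OnGameStateChanged only when the value changes.
; NextStage increments the index and broadcasts OnNextStage, capped at the last stage defined by the game mode's NumStages.
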(event EventBeginPlay
  (CallFunction|UpdateGameState "NewEnumerator3")
  (Variables|Default|SetStageIndex 0))

(fn ConstructionScript)

(fn UpdateGameState
  (params (GameState :type E_Gamestate%20Enum :default "NewEnumerator0"))
  (if (Utilities|Enum|NotEqual(Enum) GameState (Variables|Default|GetGameState))
    (bind _output_get (Variables|Default|SetGameState GameState))
    (Default|CallOnGameStateChanged _output_get)))

(fn NextStage
  (if (<= (+ (Variables|Default|GetStageIndex) 1) (- (Variables|/Game/Blueprints/Game/BP_Gamemode.BP_Gamemode_C|GetNumStages (CallFunction|GetBPGameMode)) 1))
    (Variables|Default|SetStageIndex (+ (Variables|Default|GetStageIndex) 1))
    (Default|CallOnNextStage)))