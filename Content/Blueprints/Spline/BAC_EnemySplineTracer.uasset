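; Spline tracer component for enemies that keeps them on the same spline the Dragoon is tracing.
; On BeginPlay it binds to the Dragoon tracer's new-spline event and traces each new spline it receives.
; It overrides GetTracedTransform to add a settable offset to the parent's location, leaving rotation and scale untouched.
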(event Custom|OnDragoonSplineUpdated
  (params (NewSpline :type BP%20Spline%20Path%20Object%20Reference))
  (CallFunction|TraceSpline NewSpline))

(event EventBeginPlay
  (EventDispatchers|AssignOnTraceNewSpline (Variables|/Game/Blueprints/Player/BP_Dragoon.BP_Dragoon_C|GetBAC_DragonSplineTracer (CallFunction|GetDragoon)) (delegate Custom|OnDragoonSplineUpdated)))

(fn GetTracedTransform
  (bind _transform (|CallParentFunction))
  (return (Math|Transform|MakeTransform (+ (Variables|Default|GetAdditionalOffset) (.location _transform)) (.rotation _transform) (.scale _transform))))

(fn UpdateAdditionalOffset
  (params (AdditionalOffset :type Vector))
  (Variables|Default|SetAdditionalOffset AdditionalOffset))