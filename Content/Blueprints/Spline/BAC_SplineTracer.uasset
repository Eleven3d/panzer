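; BAC_SplineTracer is an actor component that moves its owner along a spline, restarting on looping splines or otherwise stopping and signalling arrival.
; Each tick sweeps the owner to the constant-velocity spline transform at unit scale, then advances position and fires an update.
; Normalized time divides that speed-scaled position by spline length over speed, so pace grows with speed squared.
; GetVelocity returns displacement since the last tick's starting location, not divided by delta time.
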(event EventTick
  (params (DeltaSeconds :type Float%20%28single-precision%29))
  (Variables|Default|SetPreviousWorldLocation (Transformation|GetActorLocation (Components|GetOwner)))
  (CallFunction|UpdateSplineTransform)
  (Variables|Spline|SetPositionOnSpline (+ (Variables|Spline|GetPositionOnSpline) (* (Variables|Spline|GetTraceSpeed) (Utilities|Time|GetWorldDeltaSeconds))))
  (Default|CallOnSplineTraceUpdate)
  (if (>= (SplineMovement|CalculateTime) 1.0)
    (if (Variables|/Game/Blueprints/Spline/BP_SplinePath.BP_SplinePath_C|GetLooping (Variables|Spline|GetSplineToTrace))
      (SplineMovement|TraceSpline (Variables|Spline|GetSplineToTrace))
      (else
        (SplineMovement|SplineDestinationReached)))))

(event EventBeginPlay
  (Actor|Tick|AddTickPrerequisiteActor (Components|GetOwner)))

(fn TraceSpline
  (params (SplineToTrace :type BP%20Spline%20Path%20Object%20Reference))
  (Variables|Spline|SetSplineToTrace SplineToTrace)
  (Variables|Spline|SetPositionOnSpline 0.0)
  (Components|Tick|SetComponentTickEnabled true))

(fn CalculateTime
  (return (Math|Float|MapRangeClamped (Variables|Spline|GetPositionOnSpline) 0.0 (/ (Spline|GetSplineLength (Variables|/Game/Blueprints/Spline/BP_SplinePath.BP_SplinePath_C|GetSpline (Variables|Spline|GetSplineToTrace))) (Variables|Spline|GetTraceSpeed)) 0.0 1.0)))

(fn SetTraceSpeed
  (params (TraceSpeed :type Float%20%28single-precision%29))
  (Variables|Spline|SetTraceSpeed TraceSpeed))

(fn SplineDestinationReached
  (Components|Tick|SetComponentTickEnabled false)
  (Default|CallOnSplineDestinationReached))

(fn GetTracedTransform
  (bind _time (SplineMovement|CalculateTime))
  (bind _splinetotrace (Variables|Spline|GetSplineToTrace))
  (bind _spline (Variables|/Game/Blueprints/Spline/BP_SplinePath.BP_SplinePath_C|GetSpline _splinetotrace))
  (bind _returnvalue (Spline|GetTransformatTime _spline _time "World" true false))
  (return (Math|Transform|MakeTransform (.location _returnvalue) (.rotation _returnvalue) "1,1,1")))

(fn GetVelocity
  (return (- (Transformation|GetActorLocation (Components|GetOwner)) (Variables|Default|GetPreviousWorldLocation))))

(fn UpdateSplineTransform
  (Transformation|SetActorTransform (Components|GetOwner) (SplineMovement|GetTracedTransform) true))

(fn StopTracingSpline
  (Components|Tick|SetComponentTickEnabled false)
  (Variables|Spline|SetSplineToTrace 0)
  (Variables|Spline|SetPositionOnSpline 0.0))