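; Spline tracer component, apparently for a dragon, that lets the player's view direction shift the traced point away from the spline.
; Each tick it accumulates the player camera's forward vector, scaled by speed and delta time, into an offset clamped per axis to the offset radius, forming a box rather than a sphere.
; The GetTracedTransform override adds this world-axis offset to the parent's location, keeping rotation and scale.
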(event EventTick
  (params (DeltaSeconds :type Float%20%28single-precision%29))
  (bind _splineoffsetradius (Variables|Spline|GetSplineOffsetRadius))
  (|CallParentFunction DeltaSeconds)
  (Variables|Spline|SetCurrentSplineOffset (CallFunction|ClampVector (+ (* (Math|Rotator|GetRotationXVector (Camera|GetCameraRotation (Game|GetPlayerCameraManager 0))) (* (Variables|Spline|GetSplineOffsetSpeed) (Utilities|Time|GetWorldDeltaSeconds))) (Variables|Spline|GetCurrentSplineOffset)) (Math|Conversions|ToVector(Float) (CallFunction|InvertFloat _splineoffsetradius)) (Math|Conversions|ToVector(Float) _splineoffsetradius))))

(fn GetTracedTransform
  (bind _transform (|CallParentFunction))
  (return (Math|Transform|MakeTransform (+ (.location _transform) (Variables|Spline|GetCurrentSplineOffset)) (.rotation _transform) (.scale _transform))))