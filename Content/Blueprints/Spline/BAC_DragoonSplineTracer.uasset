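; Spline tracer component for the Dragoon, extending a parent tracer with a movable offset from the traced spline.
; TraceSpline runs the parent logic, then calls OnTraceNewSpline with the new spline.
; GetTracedTransform adds CurrentSplineOffset to the parent's location without rotating it, keeping rotation and scale.
; SetCurrentSplineOffset accumulates offsets, clamping each axis to plus or minus SplineOffsetRadius, so the bounds form a box.
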(event EventTraceSpline
  (params (SplineToTrace :type BP%20Spline%20Path%20Object%20Reference))
  (|CallParentFunction SplineToTrace)
  (Default|CallOnTraceNewSpline SplineToTrace))

(fn GetTracedTransform
  (bind _transform (|CallParentFunction))
  (return (Math|Transform|MakeTransform (+ (.location _transform) (Variables|Spline|GetCurrentSplineOffset)) (.rotation _transform) (.scale _transform))))

(fn SetCurrentSplineOffset
  (params (AdditionalOffset :type Vector))
  (bind _splineoffsetradius (Variables|Spline|GetSplineOffsetRadius))
  (Variables|Spline|SetCurrentSplineOffset (CallFunction|ClampVector (+ AdditionalOffset (Variables|Spline|GetCurrentSplineOffset)) (Math|Conversions|ToVector(Float) (CallFunction|InvertFloat _splineoffsetradius)) (Math|Conversions|ToVector(Float) _splineoffsetradius))))