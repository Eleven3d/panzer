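; BP_TentacleEnemy is a tentacle enemy unit that animates its spline offset once the Dragoon starts tracing a new spline.
; On BeginPlay it listens to the dragon spline tracer's new-spline event, then unbinds after the first trigger, making it a one-shot.
; That trigger plays the EnemyOffset timeline, whose curve feeds the additional offset of its own enemy spline tracer component.
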(event OnTimelineUpdated(EnemyOffset)
  (params (CurrentTime :type Float%20%28single-precision%29) (CurveValue :type Vector :default "0, 0, 0") (Direction :type ETimelineDirection%20Enum :default "Forward"))
  (Default|UpdateAdditionalOffset (Variables|Default|GetBAC_EnemySplineTracer) CurveValue))

(event Custom|OnNewDragonSpline
  (params (NewSpline :type BP%20Spline%20Path%20Object%20Reference))
  (EventDispatchers|UnbindEventfromOnTraceNewSpline (Variables|/Game/Blueprints/Player/BP_Dragoon.BP_Dragoon_C|GetBAC_DragonSplineTracer (CallFunction|GetDragoon)) (delegate Custom|OnNewDragonSpline))
  (Default|Play (Variables|Default|GetEnemyOffset)))

(event EventBeginPlay
  (EventDispatchers|AssignOnTraceNewSpline (Variables|/Game/Blueprints/Player/BP_Dragoon.BP_Dragoon_C|GetBAC_DragonSplineTracer (CallFunction|GetDragoon)) (EventDispatchers|CreateEvent :!event Custom|OnNewDragonSpline)))

(fn ConstructionScript
  (|CallParentFunction))