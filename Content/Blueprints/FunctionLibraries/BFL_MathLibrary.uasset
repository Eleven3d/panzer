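; Blueprint function library of small float and vector math helpers.
; ClampVector clamps each axis to its own bounds and returns three separate floats, while InvertFloat flips a float's sign.
; AddVector and AddFloat write the sum back into the target by reference and also return it.
; ClampFloatChecked adds a WasClamped flag to the clamp, which also reads true on exact bounds because its range check is exclusive.
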(fn ClampVector
  (params (VectorToClamp :type Vector) (MinClampValues :type Vector) (MaxClampValues :type Vector))
  (return (Math|Vector|MakeVector (Math|Float|Clamp(Float) (.x VectorToClamp) (.x MinClampValues) (.x MaxClampValues)) (Math|Float|Clamp(Float) (.y VectorToClamp) (.y MinClampValues) (.y MaxClampValues)) (Math|Float|Clamp(Float) (.z VectorToClamp) (.z MinClampValues) (.z MaxClampValues)))))

(fn InvertFloat
  (params (TargetFloat :type Float%20%28single-precision%29))
  (return (* TargetFloat -1.0)))

(fn AddVector
  (params (TargetVector :type Vector%20%28by%20ref%29) (AddedValue :type Vector))
  (bind _returnvalue (+ TargetVector AddedValue))
  (|SetBy-RefVar TargetVector _returnvalue)
  (return _returnvalue))

(fn AddFloat
  (params (TargetFloat :type Float%20%28single-precision%29%20%28by%20ref%29) (AddedValue :type Float%20%28single-precision%29))
  (bind _returnvalue (+ TargetFloat AddedValue))
  (|SetBy-RefVar TargetFloat _returnvalue)
  (return _returnvalue))

(fn ClampFloatChecked
  (params (Value :type Float%20%28single-precision%29) (Min :type Float%20%28single-precision%29) (Max :type Float%20%28single-precision%29))
  (return (Math|Float|Clamp(Float) Value Min Max) (not (Math|Float|InRange(Float) Value Min Max false false))))