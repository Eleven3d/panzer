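; Blueprint function library that looks up one of the player pawn's motion controller components by its motion source.
; GetMotionController casts player 0's pawn to BP_PlayerPawn and iterates its BSC_MotionController components.
; It returns the first whose MotionSource matches the input, or prints an on-screen warning when none is found.
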(fn GetMotionController
  (params (MotionSource :type Name))
  (LocalVariables|SetSource MotionSource)
  (bind _asbp_player_pawn (Utilities|Casting|CastToBP_PlayerPawn (Game|Player|GetPlayerPawn 0)))
  (for _array_element (Actor|GetComponentsByClass _asbp_player_pawn "/Game/Blueprints/Player/BSC_MotionController.BSC_MotionController_C")
    (if (Utilities|Name|Equal(Name) (Variables|/Script/HeadMountedDisplay.MotionControllerComponent|GetMotionSource _array_element) (LocalVariables|GetSource))
      (return _array_element)))
  (Development|PrintString 0 "No valid motion controller was found. Enter a valid name." true false)
  (return 0))